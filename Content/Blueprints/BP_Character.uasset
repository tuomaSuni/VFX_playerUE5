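; Animation showcase character with an orbit-and-zoom spring arm camera and a Settings HUD that Tab toggles.
; Functions step through animations by index, zeroing it before a short timer sets the next and updates the HUD label from a table.
; Autoplay exchanges the current index with ABP_Character.
; Other functions swap weapon meshes or switch Default, Toon and Black-and-White looks via post-process volumes and sky actors picked by array order.
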(event Input|EnhancedActionEvents|EnhancedInputActionLeft
  (params (ActionValue :type Boolean) (ElapsedSeconds :type Float%20%28double-precision%29) (TriggeredSeconds :type Float%20%28double-precision%29) (InputAction :type Input%20Action%20Object%20Reference :default "/Game/System/Inputs/Left.Left"))
  ;[1 1 1] Animations
  (:Triggered
    (Transformation|AddWorldRotation (Variables|Default|GetSpringArm) "0.000000,1.000000,0.000000" false false :!label _label))
  (:Ongoing
    (goto _label)))

(event Input|EnhancedActionEvents|EnhancedInputActionRight
  (params (ActionValue :type Boolean) (ElapsedSeconds :type Float%20%28double-precision%29) (TriggeredSeconds :type Float%20%28double-precision%29) (InputAction :type Input%20Action%20Object%20Reference :default "/Game/System/Inputs/Right.Right"))
  ;[1 1 1] Animations
  (:Triggered
    (Transformation|AddWorldRotation (Variables|Default|GetSpringArm) "0.000000,-1.000000,0.000000" false false :!label _label))
  (:Ongoing
    (goto _label)))

(event Input|EnhancedActionEvents|EnhancedInputActionUp
  (params (ActionValue :type Boolean) (ElapsedSeconds :type Float%20%28double-precision%29) (TriggeredSeconds :type Float%20%28double-precision%29) (InputAction :type Input%20Action%20Object%20Reference :default "/Game/System/Inputs/Up.Up"))
  (bind _springarm (Variables|Default|GetSpringArm))
  ;[1 1 1] Camera Logic
  (:Triggered
    (if (> (.pitch (Transformation|GetWorldRotation _springarm)) -9e+01) :!label _label
      (Transformation|AddLocalRotation _springarm "-1.000000,0.000000,0.000000" false false)))
  (:Ongoing
    (goto _label)))

(event Input|EnhancedActionEvents|EnhancedInputActionDown
  (params (ActionValue :type Boolean) (ElapsedSeconds :type Float%20%28double-precision%29) (TriggeredSeconds :type Float%20%28double-precision%29) (InputAction :type Input%20Action%20Object%20Reference :default "/Game/System/Inputs/Down.Down"))
  ;[1 1 1] Camera Logic
  (:Triggered
    (if (< (.pitch (Transformation|GetWorldRotation (Variables|Default|GetSpringArm))) 4.0) :!label _label
      (Transformation|AddLocalRotation (Variables|Default|GetSpringArm) "1.000000,0.000000,0.000000" false false)))
  (:Ongoing
    (goto _label)))

(event EventBeginPlay
  ;[1 1 1] Initialization
  (bind _asplayer_controller (Utilities|Casting|CastToPlayerController (Pawn|GetController)))
  (Utilities|IsValid (PlayerController|LocalPlayerSubsystems|GetEnhancedInputLocalPlayerSubsystem _asplayer_controller)
    (:Is%20Valid
      (Input|AddMappingContext (PlayerController|LocalPlayerSubsystems|GetEnhancedInputLocalPlayerSubsystem _asplayer_controller) "/Game/System/IMC.IMC" 0 "(bIgnoreAllPressedKeysUntilRelease=True,bForceImmediately=False,bNotifyUserSettings=False)")
      (bind _outactors (Actor|GetAllActorsOfClass "/Game/GoodSky/Blueprint/BP_GoodSky.BP_GoodSky_C"))
      (Rendering|SetActorHiddenInGame (Utilities|Array|Get(acopy) _outactors 1) true)
      (bind _returnvalue (UserInterface|CreateWidget "/Game/System/UI/Settings.Settings_C"))
      (bind _output_get (Variables|Default|SetHUD _returnvalue))
      (UserInterface|Viewport|AddtoViewport _output_get 0)
      (Variables|/Script/Engine.PlayerController|SetbShowMouseCursor (Game|GetPlayerController 0) true)
      (Variables|/Game/System/UI/Settings.Settings_C|SetplayingAnimationText (Variables|Default|GetHUD) "Idle"))))

(event Input|MouseEvents|MouseWheelAxis
  (params (AxisValue :type Float%20%28single-precision%29))
  ;[1 1 1] Camera Logic
  (Variables|Default|Setlength (Math|Float|Clamp(Float) (+ (* AxisValue -2e+01) (Variables|/Script/Engine.SpringArmComponent|GetTargetArmLength (Variables|Default|GetSpringArm))) 3e+02 1.7e+03))
  (Variables|/Script/Engine.SpringArmComponent|SetTargetArmLength (Variables|Default|GetSpringArm) (Math|Float|Clamp(Float) (+ (* AxisValue -2e+01) (Variables|/Script/Engine.SpringArmComponent|GetTargetArmLength (Variables|Default|GetSpringArm))) 3e+02 1.7e+03)))

(event Input|KeyboardEvents|Tab
  (params (Key :type Key%20Structure))
  (bind _hud (Variables|Default|GetHUD))
  (:Pressed
    (if (Class|Widget|GetIsEnabled _hud)
      (Widget|SetIsEnabled _hud false)
      (Widget|SetRenderOpacity _hud 0.0)
      (else
        (Widget|SetIsEnabled _hud true)
        (Widget|SetRenderOpacity _hud 1.0)))))

(fn ConstructionScript)

(fn Equip3
  (Rendering|SetVisibility (Variables|Default|GetSword_R) true false)
  (Rendering|SetVisibility (Variables|Default|Get2-Handed) false false))

(fn Equip2
  (Rendering|SetVisibility (Variables|Default|Get2-Handed) true false)
  (Components|StaticMesh|SetStaticMesh (Variables|Default|Get2-Handed) "/Game/Weapon_Pack/Mesh/Weapons/Weapons_Kit/SM_Sickle.SM_Sickle")
  (Rendering|SetVisibility (Variables|Default|GetSword_R) false false))

(fn Equip1
  (Rendering|SetVisibility (Variables|Default|Get2-Handed) true false)
  (Components|StaticMesh|SetStaticMesh (Variables|Default|Get2-Handed) "/Game/Weapon_Pack/Mesh/Weapons/Weapons_Kit/SM_Spear.SM_Spear")
  (Rendering|SetVisibility (Variables|Default|GetSword_R) false false))

(fn RightBegin
  (bind _autoplay (Variables|Default|GetautoPlay))
  (bind _returnvalue (!= _autoplay true))
  (if (and (!= (Variables|Default|Getcurrent_Float) 12.0) _returnvalue)
    (Variables|Default|Setsaved_Float (Variables|Default|Getcurrent_Float))
    (Variables|Default|Setcurrent_Float 0.0)
    (Utilities|Time|SetTimerbyFunctionName 0 "RightEnd" 0.02)
    (elif _returnvalue
      (Variables|Default|Setsaved_Float 0.0)
      (Variables|Default|Setcurrent_Float 0.0)
      (Variables|/Game/System/UI/Settings.Settings_C|SetplayingAnimationText (Variables|Default|GetHUD) (Utilities|Text|ToText(String) (Utilities|String|Append "currently playing: " "Idle"))))))

(fn LeftBegin
  (bind _autoplay (Variables|Default|GetautoPlay))
  (bind _returnvalue (!= _autoplay true))
  (if (and (!= (Variables|Default|Getcurrent_Float) 0.0) _returnvalue)
    (Variables|Default|Setsaved_Float (Variables|Default|Getcurrent_Float))
    (Variables|Default|Setcurrent_Float 0.0)
    (Utilities|Time|SetTimerbyFunctionName 0 "LeftEnd" 0.02)
    (elif _returnvalue
      (Variables|Default|Setsaved_Float 16.0)
      (Variables|Default|Setcurrent_Float 0.0)
      (Utilities|Time|SetTimerbyFunctionName 0 "LeftEnd" 0.02))))

(fn RightEnd
  (bind _result (Math|Float|IncrementFloat (Variables|Default|Getsaved_Float))
    (:%20%20
      (bind _output_get (Variables|Default|Setcurrent_Float _result))
      (Variables|/Game/System/UI/Settings.Settings_C|SetplayingAnimationText (Variables|Default|GetHUD) (Utilities|Text|ToText(String) (.key (.Value (Utilities|Map|Find (Variables|Default|Gettable) _output_get))))))))

(fn LeftEnd
  (bind _result (Math|Float|DecrementFloat (Variables|Default|Getsaved_Float))
    (:%20%20
      (bind _output_get (Variables|Default|Setcurrent_Float _result))
      (if (!= (Variables|Default|Getcurrent_Float) 0.0)
        (Variables|/Game/System/UI/Settings.Settings_C|SetplayingAnimationText (Variables|Default|GetHUD) (Utilities|Text|ToText(String) (.key (.Value (Utilities|Map|Find (Variables|Default|Gettable) _output_get)))))
        (else
          (Variables|/Game/System/UI/Settings.Settings_C|SetplayingAnimationText (Variables|Default|GetHUD) (Utilities|Text|ToText(String) (.key (.Value (Utilities|Map|Find (Variables|Default|Gettable) 0.0))))))))))

(fn SetAutoplay
  (bind _asabp_character (Utilities|Casting|CastToABP_Character (Components|SkeletalMesh|GetAnimInstance (Variables|Default|GetSkeletalMesh))))
  (if (== (Variables|Default|Getcurrent_Float) 0.0)
    (Variables|Default|Setcurrent_Float 1.0)
    (Variables|/Game/Animations/ABP_Character.ABP_Character_C|Setsaved_Anim _asabp_character 1.0))
  (if (Variables|Default|GetautoPlay)
    (Variables|Default|SetautoPlay false)
    (Variables|Default|Setcurrent_Float (Variables|/Game/Animations/ABP_Character.ABP_Character_C|Getcurrent_Anim _asabp_character))
    (else
      (Variables|Default|SetautoPlay true)
      (Variables|/Game/Animations/ABP_Character.ABP_Character_C|Setcurrent_Anim _asabp_character (Variables|Default|Getcurrent_Float)))))

(fn Replay
  (if (!= (Variables|Default|GetautoPlay) true)
    (Variables|Default|Setsaved_Float (Variables|Default|Getcurrent_Float))
    (Variables|Default|Setcurrent_Float 0.0)
    (Utilities|Time|SetTimerbyFunctionName 0 "" 0.02)))

(fn SetStyleBlackandWhite
  (bind _outactors (Actor|GetAllActorsOfClass "/Script/Engine.PostProcessVolume"))
  (Variables|/Script/Engine.PostProcessVolume|SetbUnbound (Utilities|Array|Get(acopy) _outactors) false)
  (Variables|/Script/Engine.PostProcessVolume|SetbUnbound (Utilities|Array|Get(acopy) _outactors 1) true)
  (Actor|GetAllActorsOfClass "/Game/GoodSky/Blueprint/BP_GoodSky.BP_GoodSky_C")
  (bind _outactors_2 (Actor|GetAllActorsOfClass "/Game/GoodSky/Blueprint/BP_GoodSky.BP_GoodSky_C"))
  (Rendering|SetActorHiddenInGame (Utilities|Array|Get(acopy) _outactors_2) true)
  (Rendering|SetActorHiddenInGame (Utilities|Array|Get(acopy) _outactors_2 1) false))

(fn SetStyleToon
  (bind _outactors (Actor|GetAllActorsOfClass "/Script/Engine.PostProcessVolume"))
  (Variables|/Script/Engine.PostProcessVolume|SetbUnbound (Utilities|Array|Get(acopy) _outactors) true)
  (Variables|/Script/Engine.PostProcessVolume|SetbUnbound (Utilities|Array|Get(acopy) _outactors 1) false)
  (bind _outactors_2 (Actor|GetAllActorsOfClass "/Game/GoodSky/Blueprint/BP_GoodSky.BP_GoodSky_C"))
  (Rendering|SetActorHiddenInGame (Utilities|Array|Get(acopy) _outactors_2) false)
  (Rendering|SetActorHiddenInGame (Utilities|Array|Get(acopy) _outactors_2 1) true))

(fn SetStyleDefault
  (bind _outactors (Actor|GetAllActorsOfClass "/Script/Engine.PostProcessVolume"))
  (Variables|/Script/Engine.PostProcessVolume|SetbUnbound (Utilities|Array|Get(acopy) _outactors) false)
  (Variables|/Script/Engine.PostProcessVolume|SetbUnbound (Utilities|Array|Get(acopy) _outactors 1) false)
  (bind _outactors_2 (Actor|GetAllActorsOfClass "/Game/GoodSky/Blueprint/BP_GoodSky.BP_GoodSky_C"))
  (Rendering|SetActorHiddenInGame (Utilities|Array|Get(acopy) _outactors_2) false)
  (Rendering|SetActorHiddenInGame (Utilities|Array|Get(acopy) _outactors_2 1) true))